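; A door component that toggles its owning actor between open and closed positions whenever its Open event fires.
; Open slides the owner's root component by HeightToOpen, or back by the same offset, using an eased, latent MoveComponentTo with unchanged rotation.
; A Moving flag ignores calls during the slow move, and IsOpen tracks which direction the next call takes.
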(event `self.ReceiveTick`
  (params (DeltaSeconds :type "Float (single-precision)")))

(event `self.Open`
  (bind _returnvalue (`self.GetOwner` self))
  (bind _returnvalue_2 (`Actor.K2_GetActorRotation` _returnvalue))
  (bind _returnvalue_3 (`Actor.K2_GetActorLocation` _returnvalue))
  (bind _rootcomponent (`Actor.RootComponent` _returnvalue))
  (if (not (`self.Moving`))
    (if (`self.isOpen`)
      (set `self.Moving` true)
      (`KismetSystemLibrary.MoveComponentTo` _rootcomponent (+ _returnvalue_3 (* (`self.HeightToOpen`) -1)) _returnvalue_2 true false 10.0)
      (set `self.isOpen` false)
      (else
        (set `self.Moving` true)
        (`KismetSystemLibrary.MoveComponentTo` _rootcomponent (+ _returnvalue_3 (`self.HeightToOpen`)) _returnvalue_2 true false 10.0)
        (set `self.isOpen` true)))
    (set `self.Moving` false)))